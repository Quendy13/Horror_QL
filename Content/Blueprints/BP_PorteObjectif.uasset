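; BP_PorteObjectif is the objective door that ends the game when the player opens it with a key.
; It caches the first-person character on BeginPlay, and Interact checks that character's HasKey, playing a sound at the door if it is false.
; With the key, a timeline drives the door's absolute world yaw while disabling player input on each update, then calls EndGame on the character when finished.
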(event `self.ReceiveBeginPlay`
  (bind _asbp_first_person_character (cast `/Game/Blueprints/Characters/Player/FirstPerson/BP_FirstPersonCharacter` (`GameplayStatics.GetPlayerCharacter` 0))
    (:`then`
      (set `self.CharacterRef` _asbp_first_person_character))
    (:`CastFailed`
      (`KismetSystemLibrary.PrintString` "Cast Error: First Person Character in BP_PorteObjectif" true true (struct :`R` 1.0 :`A` 1.0)))))

(event `/Game/Blueprints/Interfaces/BPI_Interact.Interact`
  (if (`/Game/Blueprints/Characters/Player/FirstPerson/BP_FirstPersonCharacter.bHasKey` (`self.CharacterRef`))
    (`self.DoorOpen`)
    (else
      (`GameplayStatics.PlaySoundAtLocation` null (`SceneComponent.K2_GetComponentLocation` (`self.Door`)) (struct) 1.0 1.0 0.0 null null null null))))

(event `DoorOpen`
  (bind _door (`self.Door`))
  (bind (_returnvalue_roll _returnvalue_pitch) (`KismetMathLibrary.BreakRotator` (`SceneComponent.K2_GetComponentRotation` _door)))
  (`GameplayStatics.PlaySound2D` "/Game/Sounds/DoorOpening.DoorOpening" 1.0 1.0 0.0 null null)
  (bind (_direction _opening) (`Timeline|DoorOpening`)
    (:`Update`
      (`SceneComponent.K2_SetWorldRotation` _door (`KismetMathLibrary.MakeRotator` _returnvalue_roll _returnvalue_pitch _opening) false false)
      (`self.DisableInput` (`self.CharacterRef`) (`GameplayStatics.GetPlayerController` 0)))
    (:`Finished`
      (`/Game/Blueprints/Characters/Player/FirstPerson/BP_FirstPersonCharacter.EndGame` (`self.CharacterRef`)))))

(fn `UserConstructionScript`)