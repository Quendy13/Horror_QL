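; BP_StationEnigme is an interactable puzzle chest where the player places three collected statuettes to unlock a key.
; Each Interact spends one statue from the character's Collectibles map and reveals the next statuette mesh with a sound, or plays a failure sound.
; The third statue triggers chained Latch and Cap timelines that open the chest.
; Later interaction hides the key, sets the player's HasKey and increments its collectible count, once only.
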(event `self.ReceiveBeginPlay`
  ; Enregistre une référence au character
  (bind _asbp_first_person_character (cast `/Game/Blueprints/Characters/Player/FirstPerson/BP_FirstPersonCharacter` (`GameplayStatics.GetPlayerCharacter` 0))
    (:`then`
      (set `self.CharacterRef` _asbp_first_person_character))
    (:`CastFailed`
      (`KismetSystemLibrary.PrintString` "Cast Failed: First PersonCharacter in BP_StationEnigme" true true (struct :`R` 1.0 :`A` 1.0)))))

(event `/Game/Blueprints/Interfaces/BPI_Interact.Interact`
  ; Évènements d'interaction
  (if (`self.bHasAllStatues`)
    (`self.RetrieveKey`)
    (else
      (`self.InsertStatue`))))

(event `InsertStatue`
  (bind _collectibles (`/Game/Blueprints/Characters/Player/FirstPerson/BP_FirstPersonCharacter.Collectibles` (`self.CharacterRef`)))
  (bind _value (`BlueprintMapLibrary.Map_Find` _collectibles "NewEnumerator0"))
  ; Insertion des statues
  (if (> _value 0)
    (bind _result (`/Engine/EditorBlueprintResources/StandardMacros.DecrementInt` _value)
      (:`  `
        (`BlueprintMapLibrary.Map_Add` _collectibles "NewEnumerator0" _result)
        (bind _result_2 (`/Engine/EditorBlueprintResources/StandardMacros.IncrementInt` (`self.NbPlacedStatues`))
          (:`  `
            (switch `int` _result_2
              (:`1`
                (`StaticMeshComponent.SetStaticMesh` (`self.Statue1`) "/Game/Imports/Victorian_House/Meshes/DecorativeElements/Mesh_Statuette_01.Mesh_Statuette_01")
                (`GameplayStatics.PlaySound2D` "/Game/Sounds/PlaceStatue1.PlaceStatue1" 1.0 1.0 0.0 null null))
              (:`2`
                (`StaticMeshComponent.SetStaticMesh` (`self.Statue2`) "/Game/Imports/Victorian_House/Meshes/DecorativeElements/Mesh_Statuette_02.Mesh_Statuette_02")
                (`GameplayStatics.PlaySound2D` "/Game/Sounds/PlaceStatue2.PlaceStatue2" 1.0 1.0 0.0 null null))
              (:`3`
                (`StaticMeshComponent.SetStaticMesh` (`self.Statue3`) "/Game/Imports/Victorian_House/Meshes/DecorativeElements/Mesh_Statuette_03.Mesh_Statuette_03")
                (`GameplayStatics.PlaySound2D` "/Game/Sounds/PlaceStatue3.PlaceStatue3" 1.0 1.0 0.0 null null)
                (`self.Opening`)))))))
    (else
      (`GameplayStatics.PlaySound2D` "/Game/Sounds/PlaceNoStatue.PlaceNoStatue" 1.0 1.0 0.0 null null))))

(event `Opening`
  (bind _lacth (`self.Lacth`))
  (bind _chestcap (`self.ChestCap`))
  (bind (_returnvalue_roll _returnvalue_pitch _returnvalue_yaw) (`KismetMathLibrary.BreakRotator` (`SceneComponent.K2_GetComponentRotation` _lacth)))
  (bind (_returnvalue_roll_2 _returnvalue_pitch_2 _returnvalue_yaw_2) (`KismetMathLibrary.BreakRotator` (`SceneComponent.K2_GetComponentRotation` _chestcap)))
  ; Animation d'ouverture du coffre
  (bind (_direction _latching) (`Timeline|Latch`)
    (:`Update`
      (`SceneComponent.K2_SetWorldRotation` _lacth (`KismetMathLibrary.MakeRotator` _returnvalue_roll (* _latching 80.0) _returnvalue_yaw) false false))
    (:`Finished`
      (`GameplayStatics.PlaySound2D` "/Game/Sounds/ChestOpening.ChestOpening" 1.0 1.0 0.0 null null)
      (bind (_direction_2 _capping) (`Timeline|Cap`)
        (:`Update`
          (`SceneComponent.K2_SetWorldRotation` _chestcap (`KismetMathLibrary.MakeRotator` (* _capping -60.0) _returnvalue_pitch_2 _returnvalue_yaw_2) false false))
        (:`Finished`
          (set `self.bHasAllStatues` true))))))

(event `RetrieveKey`
  (bind _characterref (`self.CharacterRef`))
  (bind _collectibles (`/Game/Blueprints/Characters/Player/FirstPerson/BP_FirstPersonCharacter.Collectibles` _characterref))
  ; Joueur prend la clé
  (if (`self.bKeyNotRetrieved`)
    (`StaticMeshComponent.SetStaticMesh` (`self.Key`) null)
    (`GameplayStatics.PlaySound2D` "/Game/Sounds/KeyCling.KeyCling" 1.0 1.0 0.0 null null)
    (set `/Game/Blueprints/Characters/Player/FirstPerson/BP_FirstPersonCharacter.bHasKey` true _characterref)
    (bind _result (`/Engine/EditorBlueprintResources/StandardMacros.IncrementInt` (`BlueprintMapLibrary.Map_Find` _collectibles "NewEnumerator1"))
      (:`  `
        (`BlueprintMapLibrary.Map_Add` _collectibles "NewEnumerator1" _result)
        (set `self.bKeyNotRetrieved` false)))))

(fn `UserConstructionScript`)