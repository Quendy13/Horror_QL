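; BP_RockingChair is a Blueprint for a chair that rocks continuously, starting at BeginPlay.
; The Balance timeline drives the Chair component's relative roll by scaling its Balancing track, with pitch and yaw held at zero.
; Each time the timeline finishes, the Back flag flips and calls the Forward or Backward event, which plays or reverses it to keep the motion going.
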(event `self.ReceiveBeginPlay`
  (bind (_direction _balancing) (`Timeline|Balance` :!label _label)
    (:`Update`
      (`SceneComponent.K2_SetRelativeRotation` (`self.Chair`) (`KismetMathLibrary.MakeRotator` (* _balancing 20.0)) false false))
    (:`Finished`
      (if (`self.Back`)
        (set `self.Back` false)
        (`self.Forward`)
        (else
          (set `self.Back` true)
          (`self.Backward`))))))

(event `Forward`
  (goto _label))

(event `Backward`
  (goto _label :!via `Reverse`))

(fn `UserConstructionScript`)