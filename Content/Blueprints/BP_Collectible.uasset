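; BP_Collectible is a pickup actor for statuettes, keys (Clefs) and pieces that the first-person character collects.
; On BeginPlay it caches the player character and picks its static mesh from the CollectibleName type.
; Interact increments that type's count in the character's Collectibles map, sets HasKey for Clefs, then destroys the actor.
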(event `self.ReceiveBeginPlay`
  (bind _collectible (`self.Collectible`))
  (`|ExecutionSequence`
    (:`then_0`
      (bind _asbp_first_person_character (cast `/Game/Blueprints/Characters/Player/FirstPerson/BP_FirstPersonCharacter` (`GameplayStatics.GetPlayerCharacter` 0))
        (:`then`
          (set `self.CharacterRef` _asbp_first_person_character))
        (:`CastFailed`
          (`KismetSystemLibrary.PrintString` "Cast Error: First Person Character in BP_Collectible" true true (struct :`R` 1.0 :`A` 1.0)))))
    (:`then_1`
      (switch `/Game/Enum_Collectibles` (`self.CollectibleName`)
        (:`NewEnumerator0`
          (`StaticMeshComponent.SetStaticMesh` _collectible "/Game/Imports/Victorian_House/Meshes/DecorativeElements/Mesh_Statuette_02.Mesh_Statuette_02"))
        (:`NewEnumerator1`
          (`StaticMeshComponent.SetStaticMesh` _collectible "/Game/Imports/Key/SM_clef.SM_clef"))
        (:`NewEnumerator2`
          (`StaticMeshComponent.SetStaticMesh` _collectible "/Game/Imports/Victorian_House/Meshes/DecorativeElements/Mesh_ChessFigure_02.Mesh_ChessFigure_02"))))))

(event `/Game/Blueprints/Interfaces/BPI_Interact.Interact`
  (bind _collectiblename (`self.CollectibleName`))
  (bind _collectibles (`/Game/Blueprints/Characters/Player/FirstPerson/BP_FirstPersonCharacter.Collectibles` (`self.CharacterRef`)))
  (bind _result (`/Engine/EditorBlueprintResources/StandardMacros.IncrementInt` (`BlueprintMapLibrary.Map_Find` _collectibles _collectiblename))
    (:`  `
      (`BlueprintMapLibrary.Map_Add` _collectibles _collectiblename _result)
      (if (`|EnumEquality` (`self.CollectibleName`) "NewEnumerator1")
        (set `/Game/Blueprints/Characters/Player/FirstPerson/BP_FirstPersonCharacter.bHasKey` true (`self.CharacterRef`)))
      (`self.K2_DestroyActor`))))

(fn `UserConstructionScript`)